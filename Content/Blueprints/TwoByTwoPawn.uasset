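; Player pawn for a 2x2 Rubik's cube game that handles view rotation and test UI setup.
; On BeginPlay it adds the Enhanced Input mapping context, finds the cube and camera pivot by actor tag, adds a face-rotation test widget and shows the cursor.
; When not dragging, look input yaws the cube and pitches the camera pivot separately, composing rotations as quaternions.
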(event Input|EnhancedActionEvents|EnhancedInputActionIA_Look
  (params (ActionValue :type Vector%202D%20Structure) (ElapsedSeconds :type Float%20%28double-precision%29) (TriggeredSeconds :type Float%20%28double-precision%29) (InputAction :type Input%20Action%20Object%20Reference :default "/Game/Inputs/IA_Look.IA_Look"))
  (bind (_x _y) (Math|Vector2D|BreakVector2D ActionValue))
  (bind _minicuberef (Variables|Default|GetMiniCubeRef))
  (bind _rootcomponent (Variables|/Script/Engine.Actor|GetRootComponent _minicuberef))
  (if (not (Variables|Default|GetIsDragging))
    ;[0.15 0.15 0.15 0.5] 左右旋转魔方
    (Transformation|SetRelativeRotation _rootcomponent (Class|KismetMathLibrary|QuatRotator (* (Math|Conversions|ToQuaternion(Rotator) (Variables|/Script/Engine.SceneComponent|GetRelativeRotation _rootcomponent)) (Math|Conversions|ToQuaternion(Rotator) (Math|Rotator|MakeRotator 0.0 0.0 _x)))) false false)
    ;[0.15 0.15 0.15 0.5] 上下旋转镜头
    (Transformation|SetRelativeRotation (Variables|/Script/Engine.Actor|GetRootComponent (Variables|Default|GetCameraPivotRef)) (Class|KismetMathLibrary|QuatRotator (* (Math|Conversions|ToQuaternion(Rotator) (Variables|/Script/Engine.SceneComponent|GetRelativeRotation (Variables|/Script/Engine.Actor|GetRootComponent (Variables|Default|GetCameraPivotRef)))) (Math|Conversions|ToQuaternion(Rotator) (Math|Rotator|MakeRotator 0.0 _y 0.0)))) false false)))

(event EventBeginPlay
  (bind _astwo_by_two_player_controller (Utilities|Casting|CastToTwoByTwoPlayerController (Game|GetPlayerController 0) :!pinned true)) ; 在Pawn里边获取控制器，绑定增强输入系统的Input Mapping Context
  (bind _output_get (Variables|Default|SetCubePlayerControllerRef _astwo_by_two_player_controller))
  (Input|AddMappingContext (PlayerController|LocalPlayerSubsystems|GetEnhancedInputLocalPlayerSubsystem _output_get) "/Game/Inputs/IMC_RubikCube.IMC_RubikCube" 0 "(bIgnoreAllPressedKeysUntilRelease=True,bForceImmediately=False,bNotifyUserSettings=False)" :!pinned true) ; IMC_RubiCube里边，鼠标/触摸屏控制魔方6个面、镜头和整个魔方的旋转
  (bind _outactors (Actor|GetAllActorswithTag "MiniCube" :!pinned true)) ; 魔方已添加Tag：MiniCube，方便在Pawn里边找到魔方并存个引用
  (Variables|Default|SetMiniCubeRef (Utilities|Array|Get(acopy) _outactors))
  (bind _outactors_2 (Actor|GetAllActorswithTag "CameraPivot" :!pinned true)) ; 镜头已添加Tag：CameraPivot，方便在Pawn里边找到镜头并存个引用
  (Variables|Default|SetCameraPivotRef (Utilities|Array|Get(acopy) _outactors_2))
  (bind _returnvalue (UserInterface|CreateWidget "/Game/Blueprints/WBP_RotateCube.WBP_RotateCube_C")) ; 目前是测试用界面：12个按钮顺/逆时针旋转魔方6个面
  (bind _output_get_2 (Variables|Default|SetRotateCubeWidgetRef _returnvalue))
  (UserInterface|Viewport|AddtoViewport _output_get_2 0) ; 旋转魔方6个面功能已OK，隐藏测试用界面
  (Default|ShowCursor (Variables|Default|GetCubePlayerControllerRef)))

(fn ConstructionScript)